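; Placed ammo box that, on interaction, tops up the interacting character's reserve ammo from its own finite supply.
; Interact calls RefillAmmoOfType for two firearm types, giving a full or partial refill and deducting from CurrentAmmo.
; HUD update and empty-box destruction only run when a player holds the refilled gun.
; RefillPrimaryAmmo and RefillSecondaryAmmo duplicate this logic per slot but are not called here.
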(event `self.ReceiveBeginPlay`)

(event `/Game/Gameplay/WorldObjects/Interactables/BPI_Interactable.Interact`
  (params (InteractingCharacter :type "/Game/Gameplay/Characters/BP_BaseCharacter Object Reference"))
  (`self.RefillAmmoOfType` InteractingCharacter)
  (`self.RefillAmmoOfType` InteractingCharacter "NewEnumerator9"))

(fn `RefillAmmoOfType`
  (params (InteractingCharacter :type "/Game/Gameplay/Characters/BP_BaseCharacter Object Reference") (FireArmType :type "/Game/Gameplay/Enums/Enum_FireArmType Enum" :default "NewEnumerator7"))
  (locals (FireArm :type "/Game/Gameplay/WorldObjects/Equippables/Weapons/FireArms/SMBP_FireArmMaster Object Reference") (InteractingCharactor :type "/Game/Gameplay/Characters/BP_BaseCharacter Object Reference") (AmmoNeeded :type Integer))
  (bind _interactingcharactor (`local.InteractingCharactor`))
  (bind _firearm (`local.FireArm`))
  (bind _firearm_2 (`local.FireArm`))
  (bind _output_get (set `local.InteractingCharactor` InteractingCharacter))
  (bind (_firearmobject _hasfirearmoftype) (`/Game/Gameplay/Characters/BP_BaseCharacter.GetFireArmOfType` _output_get FireArmType))
  (if _hasfirearmoftype
    (bind _output_get_2 (set `local.FireArm` _firearmobject))
    (bind _output_get_3 (set `local.AmmoNeeded` (- (`/Game/Gameplay/WorldObjects/Equippables/Weapons/FireArms/SMBP_FireArmMaster.MaxReserveAmmo` _output_get_2) (`/Game/Gameplay/WorldObjects/Equippables/Weapons/FireArms/SMBP_FireArmMaster.ReserveAmmo` _output_get_2))))
    (if (> _output_get_3 0)
      (if (<= (`local.AmmoNeeded`) (`self.CurrentAmmo`))
        (set `/Game/Gameplay/WorldObjects/Equippables/Weapons/FireArms/SMBP_FireArmMaster.ReserveAmmo` (`/Game/Gameplay/WorldObjects/Equippables/Weapons/FireArms/SMBP_FireArmMaster.MaxReserveAmmo` _firearm_2) _firearm_2)
        (set `self.CurrentAmmo` (- (`self.CurrentAmmo`) (`local.AmmoNeeded`)))
        (else
          (set `/Game/Gameplay/WorldObjects/Equippables/Weapons/FireArms/SMBP_FireArmMaster.ReserveAmmo` (+ (`/Game/Gameplay/WorldObjects/Equippables/Weapons/FireArms/SMBP_FireArmMaster.ReserveAmmo` _firearm) (`self.CurrentAmmo`)) _firearm)
          (set `self.CurrentAmmo` 0)))
      (if (and (== (`local.FireArm`) (`/Game/Gameplay/Characters/BP_BaseCharacter.GetCurrentEquippable` _interactingcharactor)) (`GameplayStatics.ObjectIsA` _interactingcharactor "/Game/Gameplay/Characters/Player_FPS/BP_BasePlayer.BP_BasePlayer_C"))
        (`/Game/Gameplay/WorldObjects/Equippables/SMBP_EquipableItem.UpdateHUD` (`local.FireArm`))
        (`KismetSystemLibrary.PrintString` (`KismetStringLibrary.Conv_IntToString` (`self.CurrentAmmo`)))
        (if (< (`self.CurrentAmmo`) 1)
          (`self.K2_DestroyActor`))))))

(fn `RefillPrimaryAmmo`
  (params (Interactor :type "/Game/Gameplay/Characters/BP_BaseCharacter Object Reference"))
  (locals (InteractingCharacter :type "/Game/Gameplay/Characters/BP_BaseCharacter Object Reference") (AmmoNeeded :type Integer) (PrimaryFireArm :type "/Game/Gameplay/WorldObjects/Equippables/Weapons/FireArms/SMBP_FireArmMaster Object Reference"))
  (bind _primaryfirearm (`local.PrimaryFireArm`))
  (bind _primaryfirearm_2 (`local.PrimaryFireArm`))
  (bind _interactingcharacter (`local.InteractingCharacter`))
  (bind _output_get (set `local.InteractingCharacter` Interactor))
  (bind (_currentequippableoftype _hasequippableoftype) (`/Game/Gameplay/Characters/BP_BaseCharacter.GetEquipableOfClass` _output_get "NewEnumerator0"))
  (if _hasequippableoftype
    (bind _assmbp_fire_arm_master (cast `/Game/Gameplay/WorldObjects/Equippables/Weapons/FireArms/SMBP_FireArmMaster` _currentequippableoftype)
      (:`then`
        (set `local.PrimaryFireArm` _assmbp_fire_arm_master)
        (bind _output_get_2 (set `local.AmmoNeeded` (- (`/Game/Gameplay/WorldObjects/Equippables/Weapons/FireArms/SMBP_FireArmMaster.MaxReserveAmmo` _assmbp_fire_arm_master) (`/Game/Gameplay/WorldObjects/Equippables/Weapons/FireArms/SMBP_FireArmMaster.ReserveAmmo` _assmbp_fire_arm_master))))
        (if (> _output_get_2 0)
          (if (<= (`local.AmmoNeeded`) (`self.CurrentAmmo`))
            ; If the ammo crate has enough ammo for a full refill
            (set `/Game/Gameplay/WorldObjects/Equippables/Weapons/FireArms/SMBP_FireArmMaster.ReserveAmmo` (`/Game/Gameplay/WorldObjects/Equippables/Weapons/FireArms/SMBP_FireArmMaster.MaxReserveAmmo` _primaryfirearm) _primaryfirearm)
            (set `self.CurrentAmmo` (- (`self.CurrentAmmo`) (`local.AmmoNeeded`)))
            (else
              ; Partial refill for when box doesn't have enough ammo to do a full refill
              (set `/Game/Gameplay/WorldObjects/Equippables/Weapons/FireArms/SMBP_FireArmMaster.ReserveAmmo` (+ (`/Game/Gameplay/WorldObjects/Equippables/Weapons/FireArms/SMBP_FireArmMaster.ReserveAmmo` _primaryfirearm_2) (`self.CurrentAmmo`)) _primaryfirearm_2)
              (set `self.CurrentAmmo` 0)))
          (if (and (`GameplayStatics.ObjectIsA` (`/Game/Gameplay/Characters/BP_BaseCharacter.GetCurrentEquippable` _interactingcharacter) "/Game/Gameplay/WorldObjects/Equippables/Weapons/FireArms/PrimaryFireArms/SMBP_PrimaryGun.SMBP_PrimaryGun_C") (`GameplayStatics.ObjectIsA` _interactingcharacter "/Game/Gameplay/Characters/Player_FPS/BP_BasePlayer.BP_BasePlayer_C"))
            (`/Game/Gameplay/WorldObjects/Equippables/SMBP_EquipableItem.UpdateHUD` (`local.PrimaryFireArm`))
            (`KismetSystemLibrary.PrintString` (`KismetStringLibrary.Conv_IntToString` (`self.CurrentAmmo`)))
            (if (< (`self.CurrentAmmo`) 1)
              (`self.K2_DestroyActor`)))))
      (:`CastFailed`
        (`KismetSystemLibrary.PrintString` "Equipable of class was not a firearm")))))

(fn `RefillSecondaryAmmo`
  (params (InteractingPlayer :type "/Game/Gameplay/Characters/Player_FPS/BP_BasePlayer Object Reference"))
  (locals (AmmoNeeded :type Integer) (Secondary :type "/Game/Gameplay/WorldObjects/Equippables/Weapons/FireArms/SecondaryFireArms/SMBP_SecondaryGun Object Reference") (InteractingCharacter :type "/Game/Gameplay/Characters/BP_BaseCharacter Object Reference") (SecondaryFireArm :type "/Game/Gameplay/WorldObjects/Equippables/Weapons/FireArms/SMBP_FireArmMaster Object Reference"))
  (bind _secondaryfirearm (`local.SecondaryFireArm`))
  (bind _secondaryfirearm_2 (`local.SecondaryFireArm`))
  (bind _interactingcharacter (`local.InteractingCharacter`))
  (bind _output_get (set `local.InteractingCharacter` InteractingPlayer))
  (bind (_currentequippableoftype _hasequippableoftype) (`/Game/Gameplay/Characters/BP_BaseCharacter.GetEquipableOfClass` _output_get "NewEnumerator1"))
  (if _hasequippableoftype
    (bind _assmbp_fire_arm_master (cast `/Game/Gameplay/WorldObjects/Equippables/Weapons/FireArms/SMBP_FireArmMaster` _currentequippableoftype))
    (set `local.SecondaryFireArm` _assmbp_fire_arm_master)
    (bind _output_get_2 (set `local.AmmoNeeded` (- (`/Game/Gameplay/WorldObjects/Equippables/Weapons/FireArms/SMBP_FireArmMaster.MaxReserveAmmo` _assmbp_fire_arm_master) (`/Game/Gameplay/WorldObjects/Equippables/Weapons/FireArms/SMBP_FireArmMaster.ReserveAmmo` _assmbp_fire_arm_master))))
    (if (> _output_get_2 0)
      (if (<= (`local.AmmoNeeded`) (`self.CurrentAmmo`))
        ; If the ammo crate has enough ammo for a full refill
        (set `/Game/Gameplay/WorldObjects/Equippables/Weapons/FireArms/SMBP_FireArmMaster.ReserveAmmo` (`/Game/Gameplay/WorldObjects/Equippables/Weapons/FireArms/SMBP_FireArmMaster.MaxReserveAmmo` _secondaryfirearm) _secondaryfirearm)
        (set `self.CurrentAmmo` (- (`self.CurrentAmmo`) (`local.AmmoNeeded`)))
        (else
          ; Partial refill for when box doesn't have enough ammo to do a full refill
          (set `/Game/Gameplay/WorldObjects/Equippables/Weapons/FireArms/SMBP_FireArmMaster.ReserveAmmo` (+ (`/Game/Gameplay/WorldObjects/Equippables/Weapons/FireArms/SMBP_FireArmMaster.ReserveAmmo` _secondaryfirearm_2) (`self.CurrentAmmo`)) _secondaryfirearm_2)
          (set `self.CurrentAmmo` 0)))
      (if (and (`GameplayStatics.ObjectIsA` (`/Game/Gameplay/Characters/BP_BaseCharacter.GetCurrentEquippable` _interactingcharacter) "/Game/Gameplay/WorldObjects/Equippables/Weapons/FireArms/SecondaryFireArms/SMBP_SecondaryGun.SMBP_SecondaryGun_C") (`GameplayStatics.ObjectIsA` _interactingcharacter "/Game/Gameplay/Characters/Player_FPS/BP_BasePlayer.BP_BasePlayer_C"))
        (`/Game/Gameplay/WorldObjects/Equippables/SMBP_EquipableItem.UpdateHUD` (`local.SecondaryFireArm`))
        (`KismetSystemLibrary.PrintString` (`KismetStringLibrary.Conv_IntToString` (`self.CurrentAmmo`)))
        (if (< (`self.CurrentAmmo`) 1)
          (`self.K2_DestroyActor`))))))

(fn `UserConstructionScript`)